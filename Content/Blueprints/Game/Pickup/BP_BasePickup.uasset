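; Base pickup actor that flies to the player when touched and is then collected.
; Overlapping the Sphere with a BP_ThirdPersonCharacter fires once, saving the start location and playing PickupTimeline.
; The timeline lerps the actor toward the player's current location each update, creating a homing effect.
; When it finishes, OnPickup broadcasts the OnPickupCompleteEvent dispatcher with the player and destroys the actor.
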(event OnComponentBeginOverlap(Sphere)
  (params (OverlappedComponent :type Primitive%20Component%20Object%20Reference) (OtherActor :type Actor%20Object%20Reference) (OtherComp :type Primitive%20Component%20Object%20Reference) (OtherBodyIndex :type Integer) (bFromSweep :type Boolean) (SweepResult :type Hit%20Result%20Structure%20%28by%20ref%29))
  ;[0.1443 0.15 0.05317 0.5] When overlapped by the Player: Save starting position, animate the item flying towards the Player, then trigger the Pickup event.
  ;;[0.04522 0.15 0.15 0.5] Check if it is the Player overlapping. 'Do Once' ensures the animation doesn't trigger multiple times if the player runs back and forth.
  (bind _asbp_third_person_character (Utilities|Casting|CastToBP_ThirdPersonCharacter OtherActor))
  (Utilities|FlowControl|DoOnce false
    (:Completed
      ;;[0.15 0.02841 0.1134 0.5] Save the item's current location before it starts moving. This is used as the anchor point (A) for the movement.
      (Variables|Default|Set_StartLocation (Transformation|GetActorLocation))
      ;;[0.15 0.01987 0.01901 0.5] Update loop: Smoothly move the item from 'Start Location' to the Player's current location.
      ;; This creates a 'homing' effect as the player moves.
      (bind _alpha (Timeline|PickupTimeline Play)
        (:Update
          (Transformation|SetActorLocation (Math|Vector|Lerp(Vector) (Variables|Default|Get_StartLocation) (Transformation|GetActorLocation _asbp_third_person_character) _alpha) false false))
        (:Finished
          (CallFunction|OnPickup _asbp_third_person_character) ; When the timeline finishes (item reaches the player), \nexecute the actual pickup logic (Add Score, Destroy Actor, Play Sound, etc.).
        )))))

(fn ConstructionScript)

(fn OnPickup
  (params (Player :type BP%20Third%20Person%20Character%20Object%20Reference))
  ;[0.15 0.04815 0.1206 0.5] Notify the game that the item was collected, then destroy this object.
  (Default|CallOnPickupCompleteEvent Player)
  (Actor|DestroyActor))
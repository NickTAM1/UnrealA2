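; Actor component that keeps the player's score.
; On BeginPlay it listens on the Gameplay Message channel Player.Score.Added and passes each integer payload to AdjustScore.
; AdjustScore adds the value, clamps the total at zero and broadcasts it on Player.Score.OnScoreUpdated so listeners such as the UI can update.
; GetScore exposes the current total.
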(event EventBeginPlay
  ;[0.15 0.07909 0.04604 0.5] Start listening for 'Score Added' messages. When a message arrives, open it to get the number and update the Score.
  (bind _payload (|ListenforGameplayMessages "(TagName=\"Player.Score.Added\")" "/Game/Blueprints/Data/S_Int.S_Int" "ExactMatch") ; The first exe pin on the right fires off right away so you can continue your code.\nthe "On Message Received" is callback that fires off once the message is broadcasted
    (:OnMessageReceived
      (CallFunction|AdjustScore (Utilities|Struct|BreakS_Int _payload)))))

(fn AdjustScore
  (params (value :type Integer))
  ;[0.15 0.1162 0.05914 0.5] Adds points, prevents the score from going below zero, and tells the UI to update.
  (if (< (+ value (Variables|Default|Get_score)) 0)
    (Variables|Default|Set_score 0)
    (else
      (Variables|Default|Set_score (+ value (Variables|Default|Get_score)))))
  (Messaging|BroadcastMessage (Subsystems|GetGameplayMessageSubsystem) "(TagName=\"Player.Score.OnScoreUpdated\")" (Utilities|Struct|MakeS_Int (Variables|Default|Get_score))))

(fn GetScore
  (return (Variables|Default|Get_score)))
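; BP_Door is an interactable door that swings open and closed.
; OnInteract checks the IsOpen flag and calls OpenDoor or CloseDoor, which update the flag and play or reverse OpenCloseTimeline.
; The timeline's Alpha drives a shortest-path rotator lerp that sets DoorMesh's relative rotation between zero and a 90-degree turn.
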(event Custom|OpenDoor
  (Variables|Default|Set_isOpen true)
  (bind _alpha (Timeline|OpenCloseTimeline Play)
    (:Update
      (Transformation|SetRelativeRotation (Variables|Default|GetDoorMesh) (Math|Rotator|Lerp(Rotator) "0, 0, 0" "0.000000,90.000000,0.000000" _alpha true) false false))))

(event Custom|CloseDoor
  (Variables|Default|Set_isOpen false)
  (bind _alpha (Timeline|OpenCloseTimeline Reverse)
    (:Update
      (Transformation|SetRelativeRotation (Variables|Default|GetDoorMesh) (Math|Rotator|Lerp(Rotator) "0, 0, 0" "0.000000,90.000000,0.000000" _alpha true) false false))))

(event EventOnInteract
  (params (Player :type BP%20Third%20Person%20Character%20Object%20Reference))
  (if (Variables|Default|Get_isOpen)
    (CallFunction|CloseDoor)
    (else
      (CallFunction|OpenDoor))))

(fn ConstructionScript)